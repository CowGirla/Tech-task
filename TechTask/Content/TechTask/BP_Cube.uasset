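; BP_Cube is a networked actor that bobs up and down, pulses its glow and repeatedly shoots out BP_Sphere actors.
; On BeginPlay the authority calls server events that multicast all three looping behaviours.
; Chained timelines drive the cube's relative location and EmissiveParameter, whose RepNotify updates a dynamic material created in the construction script.
; The multicast spawn loop creates a sphere at an arrow component after each random delay.
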(event `self.ReceiveBeginPlay`
  (`/Engine/EditorBlueprintResources/ActorMacros.Switch Has Authority`
    (:`Authority`
      (`self.Server_MovementUpDown`)
      (`self.Server_Changing Emissive`)
      (`self.Server_SpawnSphere`))))

(event `Server_MovementUpDown`
  ;[1 1 1] CubeMovementUpDown
  (`self.Multicast_MovementUpDown`))

(event `Server_Changing Emissive`
  ;[1 1 1] CubeEmissiveChanging
  (`self.Multicast_Changing Emissive`))

(event `Server_SpawnSphere`
  ;[1 1 1] SphereShot
  (`self.Multicast_SpawnSphere`))

(event `Multicast_Changing Emissive`
  ;[1 1 1] CubeEmissiveChanging
  (bind (_direction _changing_emissive_parameter) (`Timeline|Changing Emissive Up` :!label _label)
    (:`Update`
      (set `self.Emissive Parameter` _changing_emissive_parameter))
    (:`Finished`
      (bind (_direction_2 _chanching_emissive_parameter) (`Timeline|Changing Emissive Down` :!via `ReverseFromEnd`)
        (:`Update`
          (set `self.Emissive Parameter` _chanching_emissive_parameter))
        (:`Finished`
          (goto _label :!via `PlayFromStart`))))))

(event `Multicast_SpawnSphere`
  ;[1 1 1] SphereShot
  (`KismetSystemLibrary.Delay` (`KismetMathLibrary.RandomFloatInRange` 1.0 3.0) :!label _label_2)
  (`|SpawnActorFromClass` "/Game/TechTask/BP_Sphere.BP_Sphere_C" (`SceneComponent.K2_GetComponentToWorld` (`self.Arrow_SphereSpawnPos`)) "AlwaysSpawn" "MultiplyWithRoot" null null)
  (goto _label_2))

(event `Multicast_MovementUpDown`
  (bind _cube (`self.Cube`))
  ;[1 1 1] CubeMovementUpDown
  (bind (_direction _moving) (`Timeline|MovingUp` :!label _label_3)
    (:`Update`
      (`SceneComponent.K2_SetRelativeLocation` _cube _moving false false))
    (:`Finished`
      (bind (_direction_2 _moving_2) (`Timeline|MovingDown` :!via `ReverseFromEnd`)
        (:`Update`
          (`SceneComponent.K2_SetRelativeLocation` _cube _moving_2 false false))
        (:`Finished`
          (goto _label_3 :!via `PlayFromStart`))))))

(fn `OnRep_Emissive Parameter`
  (`MaterialInstanceDynamic.SetScalarParameterValue` (`self.Material`) "EmissiveParam" (`self.Emissive Parameter`)))

(fn `UserConstructionScript`
  (bind _returnvalue (`PrimitiveComponent.CreateDynamicMaterialInstance` (`self.Cube`) 0 null "None"))
  (set `self.Material` _returnvalue))